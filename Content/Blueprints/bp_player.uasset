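; Player Blueprint for a grid-based game with rhythm states, tracking moves and a power meter.
; Tick drains power while the player controller is in play, and GetNewPowerValue adds an amount chosen by rhythm state while power is below its maximum.
; updateTile finds the grid square at an offset from the current coordinates in the controller's flattened 2D array and swaps its material.
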(event `resetVars`
  (set `self.moves` (`self.movesDefault`)))

(event `self.ReceiveTick`
  (params (DeltaSeconds :type "Float (single-precision)"))
  (bind _playercontrollerref (`self.playerControllerRef`))
  (`/Engine/EditorBlueprintResources/StandardMacros.IsValid` _playercontrollerref
    (:`Is Valid`
      (if (`/Game/Blueprints/controllers/bp_ctlr_player.playing?` _playercontrollerref)
        (if (> (`self.powerValue`) 0.0)
          (set `self.powerValue` (- (`self.powerValue`) (`self.powerValueDecrement`))))))))

(fn `getNewPowerValue`
  (params (currentRhythmState :type "/Game/Blueprints/enums/e_rhythmState Enum"))
  (returns (`+ Amount` :type "Float (double-precision)"))
  (bind _returnvalue (select `/Game/Blueprints/enums/e_rhythmState` currentRhythmState :`NewEnumerator0` (`self.powerValueIncrement_hit`) :`NewEnumerator2` (`self.powerValueIncrement_allowed`)))
  (if (< (`self.powerValue`) (`self.powerValueMax`))
    (set `self.powerValue` (+ (`self.powerValue`) _returnvalue))
    (return _returnvalue)))

(fn `UserConstructionScript`)