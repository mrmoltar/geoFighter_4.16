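; Grid square tile actor that highlights under the mouse cursor and flags whether the player is on it.
; Cursor-over swaps the mesh material, and cursor-out calls ResetTile to apply the default one.
; Mesh begin-overlap sets PlayerHere by casting to bp_player; it only clears when another actor begins overlapping, as there is no end-overlap handler.
; SetNewMaterial lets the tile's material be overridden.
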(event `self.StaticMesh.OnComponentBeginOverlap`
  (params (OverlappedComponent :type "PrimitiveComponent Object Reference") (OtherActor :type "Actor Object Reference") (OtherComp :type "PrimitiveComponent Object Reference") (OtherBodyIndex :type Integer) (bFromSweep :type Boolean) (SweepResult :type "HitResult Structure (by ref)"))
  (cast `/Game/Blueprints/bp_player` OtherActor
    (:`then`
      (set `self.playerHere?` true))
    (:`CastFailed`
      (set `self.playerHere?` false))))

(event `self.StaticMesh.OnBeginCursorOver`
  (params (TouchedComponent :type "PrimitiveComponent Object Reference"))
  (`PrimitiveComponent.SetMaterial` TouchedComponent 0 "/Engine/MapTemplates/Materials/BasicAsset01.BasicAsset01"))

(event `self.StaticMesh.OnEndCursorOver`
  (params (TouchedComponent :type "PrimitiveComponent Object Reference"))
  (`self.resetTile`))

(fn `resetTile`
  (`PrimitiveComponent.SetMaterial` (`self.StaticMesh`) 0 "/Engine/MapTemplates/Materials/BasicAsset02.BasicAsset02")
  (return))

(fn `setNewMaterial`
  (params (newMaterial :type "Material Object Reference"))
  (`PrimitiveComponent.SetMaterial` (`self.StaticMesh`) 0 newMaterial)
  (return))

(fn `UserConstructionScript`)