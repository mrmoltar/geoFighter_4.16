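; Player controller for a rhythm-based grid game that shows the main menu and handles click actions.
; New game spawns the square grid, rhythm, enemy and music controllers, HUD, and player on a random square.
; A Gate polled on Tick allows one action per click while moves remain.
; On-beat clicks trace under the cursor to attack or move within range, spending a move and updating power; off-beat clicks lose power.
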(event `self.ReceiveBeginPlay`
  ;[1 1 1] spawn main menu widget
  (bind _returnvalue (`|CreateWidget` "/Game/Blueprints/widgets/w_mainMenu.w_mainMenu_C"))
  (`UserWidget.AddToViewport` _returnvalue 0)
  (set `self.mainMenuRef` _returnvalue))

(event `newGame`
  ;[1 1 1] new game
  (`|ExecutionSequence`
    (:`then_0`
      (`self.spawnGrid` (`self.gridHorizontal`) (`self.gridVertical`) (+ (`self.gridSize`) (`self.gridBoarder`)))
      (`self.spawnControllers`)
      (bind _returnvalue (`|CreateWidget` "/Game/Blueprints/widgets/w_hud.w_hud_C" null (`self.rhythmControllerRef`)))
      (`UserWidget.AddToViewport` _returnvalue 0)
      (set `self.hudRef` _returnvalue))
    (:`then_1`
      (bind _playerref (`self.spawnPlayer` (`KismetMathLibrary.RandomIntegerInRange` 0 (- (`self.gridHorizontal`) 1)) 1))
      (`/Engine/EditorBlueprintResources/StandardMacros.IsValid` _playerref
        (:`Is Valid`
          (set `self.playerRef` _playerref))))))

(event `self.ReceiveTick`
  (params (DeltaSeconds :type "Float (single-precision)"))
  (bind _hitresult (`self.GetHitResultUnderCursorByChannel` "TraceTypeQuery1" true))
  (bind _playerref (`self.playerRef`))
  (bind _playerref_2 (`self.playerRef`))
  (bind _playerref_3 (`self.playerRef`))
  (bind (_returnvalue_x _returnvalue_y) (`KismetMathLibrary.BreakVector` (`self.K2_GetActorLocation` (`.HitActor` (`GameplayStatics.BreakHitResult` _hitresult)))))
  (bind (_x1 _y1) (`self.calcCoordsFromLocation` _returnvalue_x _returnvalue_y))
  ;[1 1 1] player click/tap
  (`/Engine/EditorBlueprintResources/StandardMacros.IsValid` (`self.rhythmControllerRef`)
    (:`Is Valid`
      ;;[1 1 1] open gate once on tap/click and close
      (`/Engine/EditorBlueprintResources/StandardMacros.Gate` true :!label _label
        (:`Exit`
          (`|ExecutionSequence`
            (:`then_0`
              (if (> (`/Game/Blueprints/bp_player.moves` (`self.playerRef`)) 0)
                (switch `/Game/Blueprints/enums/e_rhythmState` (`/Game/Blueprints/controllers/bp_ctlr_rhythm.rhythmState` (`self.rhythmControllerRef`))
                  (:`NewEnumerator0`
                    (`/Engine/EditorBlueprintResources/StandardMacros.IsValid` (`.HitActor` (`GameplayStatics.BreakHitResult` _hitresult)) :!label _label_2
                      (:`Is Valid`
                        (bind _asbp_grid_square (cast `/Game/Blueprints/bp_gridSquare` (`.HitActor` (`GameplayStatics.BreakHitResult` _hitresult))))
                        (bind _actorhere (`/Game/Blueprints/bp_gridSquare.actorHere` _asbp_grid_square))
                        (`/Engine/EditorBlueprintResources/StandardMacros.IsValid` _actorhere
                          (:`Is Valid`
                            ;;[1 1 1] enemy take default damage
                            (bind _asbp_enemy_parent (cast `/Game/Blueprints/enemies/bp_enemy_parent` _actorhere))
                            (if (<= (`self.GetDistanceTo` _playerref_2 _asbp_enemy_parent) (`/Game/Blueprints/bp_player.defaultAttackDistance` _playerref_2))
                              (`/Game/Blueprints/enemies/bp_enemy_parent.takeDamage` _asbp_enemy_parent (`/Game/Blueprints/bp_player.defaultDamage` (`self.playerRef`)))
                              ;;[1 1 1] set moves & power value
                              (`/Engine/EditorBlueprintResources/StandardMacros.DecrementInt` (`/Game/Blueprints/bp_player.moves` _playerref_3) :!label _label_3
                                (:`  `
                                  (`/Game/Blueprints/bp_player.getNewPowerValue` _playerref_3 (`self.rhythmState`))))))
                          (:`Is Not Valid`
                            ;;[1 1 1] move to new location
                            (bind _asbp_player (cast `/Game/Blueprints/bp_player` (`GameplayStatics.GetPlayerPawn` 0)))
                            (if (<= (`self.GetDistanceTo` _asbp_player (`.HitActor` (`GameplayStatics.BreakHitResult` _hitresult))) (`self.maxDistance`))
                              (`SceneComponent.K2_SetWorldLocation` (`/Game/Blueprints/bp_player.DefaultSceneRoot` _asbp_player) (`KismetMathLibrary.MakeVector` _returnvalue_x _returnvalue_y (`self.zOffset`)) false true)
                              (`/Game/Blueprints/bp_macroLib1.get2dArray` (`self.gridArray`) (`KismetMathLibrary.FTrunc` _returnvalue_x) (`KismetMathLibrary.FTrunc` _returnvalue_y) (`self.gridHorizontal`)
                                (:`1`
                                  (set `/Game/Blueprints/bp_player.currentCoords` (`KismetMathLibrary.MakeVector` _x1 _y1) _asbp_player)
                                  (goto _label_3)))))))))
                  (:`NewEnumerator1`
                    ;;[1 1 1] miss rhythm
                    (set `/Game/Blueprints/bp_player.powerValue` (- (`/Game/Blueprints/bp_player.powerValue` _playerref) (`/Game/Blueprints/bp_player.powerValueDecrement_miss` _playerref)) _playerref :!label _label_4)
                    (`GameplayStatics.PlaySound2D` "/Engine/EditorSounds/Notifications/CompileFailed.CompileFailed"))
                  (:`NewEnumerator2`
                    (goto _label_2))
                  (:`NewEnumerator3`
                    (goto _label_4)))))
            (:`then_1`
              (goto _label :!via `Close`))))))))

(event `Key|LeftMouseButton` :consume false
  (params (Key :type "Key Structure" :default "AnyKey"))
  ;[1 1 1] player click/tap
  ;;[1 1 1] open gate once on tap/click and close
  (:`Pressed`
    (goto _label :!via `Open`))
  (:`Released`
    (goto _label :!via `Close`)))

(fn `spawnControllers`
  (bind _returnvalue (`|SpawnActorFromClass` "/Game/Blueprints/controllers/bp_ctlr_rhythm.bp_ctlr_rhythm_C" (`KismetMathLibrary.MakeTransform` (0.0 0.0 0.0)) "Undefined" "OverrideRootScale" null 0.0 self))
  (set `self.rhythmControllerRef` _returnvalue)
  (bind _returnvalue_2 (`|SpawnActorFromClass` "/Game/Blueprints/controllers/bp_ctlr_enemy.bp_ctlr_enemy_C" (`KismetMathLibrary.MakeTransform` (0.0 0.0 0.0)) "Undefined" "OverrideRootScale" null self (`self.rhythmControllerRef`)))
  (set `self.enemyControllerRef` _returnvalue_2)
  (bind _returnvalue_3 (`|SpawnActorFromClass` "/Game/Blueprints/controllers/bp_ctlr_music.bp_ctlr_music_C" (`KismetMathLibrary.MakeTransform` (0.0 0.0 0.0)) "Undefined" "OverrideRootScale" null self _returnvalue_2 (`self.rhythmControllerRef`)))
  (set `self.musicControllerRef` _returnvalue_3)
  (return))

(fn `spawnGrid`
  (params (sizeHorizontal :type Integer) (sizeVertical :type Integer) (offset :type Integer))
  (locals (localGrid :type "Array of /Game/Blueprints/structs/struct_2dGrid Structure") (sizeX :type Integer) (sizeY :type Integer :default 0) (os :type Integer))
  (set `local.sizeX` (- sizeHorizontal 1))
  (set `local.sizeY` (- sizeVertical 1))
  (set `local.os` offset)
  ;[1 1 1] loop thru Y
  (for _index (range (+ (`local.sizeY`) 1))
    (bind _returnvalue (`KismetMathLibrary.Conv_IntToDouble` (* _index (`local.os`))))
    (bind _returnvalue_2 (`|SpawnActorFromClass` "/Game/Blueprints/bp_gridSquare.bp_gridSquare_C" (`KismetMathLibrary.MakeTransform` (`KismetMathLibrary.MakeVector` _returnvalue)) "DontSpawnIfColliding" "OverrideRootScale"))
    (`KismetArrayLibrary.Array_Add` (`self.gridArray`) _returnvalue_2)
    ;;[1 1 1] loop thru X (nested)
    (for _index_2 (range 1 (+ (`local.sizeX`) 1))
      (bind _returnvalue_3 (`|SpawnActorFromClass` "/Game/Blueprints/bp_gridSquare.bp_gridSquare_C" (`KismetMathLibrary.MakeTransform` (`KismetMathLibrary.MakeVector` _returnvalue (`KismetMathLibrary.Conv_IntToDouble` (* _index_2 (`local.os`))))) "DontSpawnIfColliding" "OverrideRootScale"))
      (`KismetArrayLibrary.Array_Add` (`self.gridArray`) _returnvalue_3)))
  (return))

(fn `spawnPlayer`
  (params (X :type Integer) (Y :type Integer))
  (returns (playerRef :type "/Game/Blueprints/bp_player Object Reference"))
  (bind _element (`/Game/Blueprints/bp_macroLib1.get2dArray` (`self.gridArray`) X Y (`self.gridHorizontal`))
    (:`1`
      (bind (_returnvalue_x _returnvalue_y) (`KismetMathLibrary.BreakVector` (`self.K2_GetActorLocation` _element)))
      (bind (_x1 _y1) (`self.calcCoordsFromLocation` _returnvalue_x _returnvalue_y))
      (bind _returnvalue (`|SpawnActorFromClass` "/Game/Blueprints/bp_player.bp_player_C" (`KismetMathLibrary.MakeTransform` (`KismetMathLibrary.MakeVector` _returnvalue_x _returnvalue_y (`self.zOffset`))) "Undefined" "OverrideRootScale" null self (`self.rhythmControllerRef`) (`KismetMathLibrary.MakeVector` _x1 _y1)))
      (return _returnvalue))))

(fn `UserConstructionScript`)