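; Enemy controller that spawns one cone and one cube enemy on the player controller's grid at BeginPlay.
; SpawnEnemyAtLocation looks up the grid square and, if occupied, recursively retries at a random position within one square of it.
; Each spawned enemy receives player, rhythm and enemy controller references, claims its square, and joins the master array and its cone, cube or cylinder array.
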(event `self.ReceiveBeginPlay`
  (`self.spawnEnemyAtLocation` "/Game/Blueprints/enemies/bp_enemy_cone.bp_enemy_cone_C" (`KismetMathLibrary.RandomIntegerInRange` 2 5) (`KismetMathLibrary.RandomIntegerInRange` 2) "NewEnumerator0")
  (`self.spawnEnemyAtLocation` "/Game/Blueprints/enemies/bp_enemy_cube.bp_enemy_cube_C" 4 5 "NewEnumerator1"))

(fn `spawnEnemyAtLocation`
  (params (enemyToSpawn :type "/Game/Blueprints/enemies/bp_enemy_parent Class Reference") (X :type Integer) (Y :type Integer) (enemyType :type "/Game/Blueprints/enums/e_enemyTypes Enum"))
  (locals (X1 :type Integer) (Y1 :type Integer) (enemyClass :type "/Game/Blueprints/enemies/bp_enemy_parent Class Reference") (localEnemyTpe :type "/Game/Blueprints/enums/e_enemyTypes Enum"))
  (bind _enemyclass (`local.enemyClass`))
  (bind _playercontrollerref (`self.playerControllerRef`))
  (bind _x1 (`local.X1`))
  (bind _y1 (`local.Y1`))
  (`|ExecutionSequence`
    (:`then_0`
      ;[1 1 1] set local vars
      (set `local.X1` X)
      (set `local.Y1` Y)
      (set `local.enemyClass` enemyToSpawn)
      (set `local.localEnemyTpe` enemyType))
    (:`then_1`
      ;[1 1 1] get grid square at XY
      (bind _element (`/Game/Blueprints/bp_macroLib1.get2dArray` (`/Game/Blueprints/controllers/bp_ctlr_player.gridArray` _playercontrollerref) (`local.X1`) (`local.Y1`) (`/Game/Blueprints/controllers/bp_ctlr_player.gridHorizontal` _playercontrollerref))
        (:`1`
          (`/Engine/EditorBlueprintResources/StandardMacros.IsValid` (`/Game/Blueprints/bp_gridSquare.actorHere` _element)
            (:`Is Valid`
              ;[1 1 1] cycle thru function if actor at spawn position
              (`self.spawnEnemyAtLocation` (`local.enemyClass`) (`KismetMathLibrary.RandomIntegerInRange` (- _x1 1) (+ _x1 1)) (`KismetMathLibrary.RandomIntegerInRange` (- _y1 1) (+ _y1 1)) (`local.localEnemyTpe`)))
            (:`Is Not Valid`
              ;[1 1 1] if no enemy actor at XY location, spawn enemy
              (bind _returnvalue (`|SpawnActorFromClass` (`local.enemyClass`) (`KismetMathLibrary.MakeTransform` (`self.K2_GetActorLocation` _element)) "Undefined" "OverrideRootScale" null (`self.playerControllerRef`) (`self.rhythmControllerRef`) self (select `/Game/Blueprints/enums/e_enemyTypes` (`local.localEnemyTpe`) :`NewEnumerator0` "NewEnumerator0" :`NewEnumerator1` "NewEnumerator1" :`NewEnumerator2` "NewEnumerator2" :!type "/Game/Blueprints/enums/e_enemyTypes Enum")))
              ;[1 1 1] add enemy to enemy array
              (`KismetArrayLibrary.Array_Add` (`self.enemyArray`) _returnvalue)
              ;[1 1 1] update grid square
              (set `/Game/Blueprints/bp_gridSquare.actorHere` _returnvalue _element)
              ;[1 1 1] add to individual enemy type array
              (if (== _enemyclass "/Game/Blueprints/enemies/bp_enemy_cone.bp_enemy_cone_C")
                (`KismetArrayLibrary.Array_Add` (`self.enemyConeArray`) _returnvalue)
                (return)
                (elif (== _enemyclass "/Game/Blueprints/enemies/bp_enemy_cube.bp_enemy_cube_C")
                  (`KismetArrayLibrary.Array_Add` (`self.enemyCubeArray`) _returnvalue)
                  (return)
                  (elif (== _enemyclass "/Game/Blueprints/enemies/bp_enemy_cylinder.bp_enemy_cylinder_C")
                    (`KismetArrayLibrary.Array_Add` (`self.enemyCylinderArray`) _returnvalue)
                    (return)
                    (else
                      (return))))))))))))

(fn `UserConstructionScript`)