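; Music controller Blueprint that plays drum sounds as 2D audio through beat-named events.
; The 1&3 event plays a kick and the 2&4 event plays a snare; the file contains no timing logic to fire them.
; The snare event also plays a camera shutter sound when the enemy controller's cone array is not empty.
; Two helper graphs, an array-length check and a decimal-flooring calculation, hold only unused nodes.
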(event `1 & 3`
  (`GameplayStatics.PlaySound2D` "/Game/Blueprints/sounds/CB_Kick.CB_Kick"))

(event `2 & 4`
  (`GameplayStatics.PlaySound2D` "/Game/Blueprints/sounds/CB_Snare.CB_Snare")
  (if (`self.arrayLength>0?` (`/Game/Blueprints/controllers/bp_ctlr_enemy.enemyConeArray` (`self.enemyControllerRef`)))
    (`GameplayStatics.PlaySound2D` "/Engine/VREditor/Sounds/UI/Camera_Shutter.Camera_Shutter")))

(fn `UserConstructionScript`)